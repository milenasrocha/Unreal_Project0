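; BP_HingeDoor is a child door Blueprint that swings open on a hinge.
; Its OnOpen override calls the parent, prints a debug string, then fires a custom event that plays a timeline scaling its Rotation track to a 90-degree relative yaw on the mesh.
; OnClose only calls the parent, so this Blueprint adds no closing animation of its own.
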(event Custom|PlayOpenAnimation
  (bind _rotation (Timeline|OpenAnimation Play)
    (:Update
      (Transformation|SetRelativeRotation (Variables|Default|GetMesh) (Math|Rotator|MakeRotator 0.0 0.0 (* _rotation 9e+01)) false false))))

(event EventBeginPlay
  (|CallParentFunction) ; This node is disabled and will not be called.\nDrag off pins to build functionality.
)

(event Collision|EventActorBeginOverlap
  (params (OtherActor :type Actor%20Object%20Reference))
  (|CallParentFunction OtherActor) ; This node is disabled and will not be called.\nDrag off pins to build functionality.
)

(event EventTick
  (params (DeltaSeconds :type Float%20%28single-precision%29))
  (|CallParentFunction DeltaSeconds) ; This node is disabled and will not be called.\nDrag off pins to build functionality.
)

(fn ConstructionScript
  (|CallParentFunction))

(fn OnClose
  (|CallParentFunction))

(fn OnOpen
  (|CallParentFunction)
  (Development|PrintString "BP_HingeDoor.Open")
  (CallFunction|PlayOpenAnimation))